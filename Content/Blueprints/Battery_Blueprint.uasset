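; Battery pickup actor that adds a battery to the player's inventory when touched.
; A sphere overlap casts the other actor to MyPawnCharacter, increments its Batteries count, and destroys the pickup.
; It then prints a pickup message, plus a reload message if the character's BatteryHealth is zero.
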(event `self.Sphere.OnComponentBeginOverlap`
  (params (OverlappedComponent :type "PrimitiveComponent Object Reference") (OtherActor :type "Actor Object Reference") (OtherComp :type "PrimitiveComponent Object Reference") (OtherBodyIndex :type Integer) (bFromSweep :type Boolean) (SweepResult :type "HitResult Structure (by ref)"))
  (bind _asmy_pawn_character (cast `/Game/Blueprints/MyPawnCharacter` OtherActor))
  (set `/Game/Blueprints/MyPawnCharacter.Batteries` (+ (`/Game/Blueprints/MyPawnCharacter.Batteries` _asmy_pawn_character) 1) _asmy_pawn_character)
  (`self.K2_DestroyActor`)
  (`KismetSystemLibrary.PrintString` (`self.pickUp Message`))
  (if (== (`/Game/Blueprints/MyPawnCharacter.Battery_Health` _asmy_pawn_character) 0)
    (`KismetSystemLibrary.PrintString` (`self.reloadMssg`))))

(fn `UserConstructionScript`)